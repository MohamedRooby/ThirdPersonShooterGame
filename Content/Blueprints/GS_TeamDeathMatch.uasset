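; Game state for team deathmatch that tracks how many members of Team A and Team B are still alive.
; DecreaseTeamNumber lowers the chosen team's count, showing a winner widget for the opposing team at zero or otherwise refreshing the HUD.
; UpdateWidget writes both counts to the HUD of player 0's third-person character, and also runs shortly after BeginPlay to set the initial display.
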(event `self.ReceiveBeginPlay`
  (`KismetSystemLibrary.Delay` 0.2)
  (`self.UpdateWidget`))

(event `DecreaseTeamNumber`
  (params (TeamA :type Boolean))
  (if TeamA
    (bind _result (`/Engine/EditorBlueprintResources/StandardMacros.DecrementInt` (`self.NumberOfTeamA_Alive`))
      (:`  `
        (if (<= _result 0)
          (bind _returnvalue (`|CreateWidget` "/Game/UI/WB_TeamWinner.WB_TeamWinner_C"))
          (`TextBlock.SetText` (`/Game/UI/WB_TeamWinner.WinnerText` _returnvalue) "TEAM B WON!")
          (`UserWidget.AddToViewport` _returnvalue 0)
          (else
            (`self.UpdateWidget` :!label _label)))))
    (else
      (bind _result_2 (`/Engine/EditorBlueprintResources/StandardMacros.DecrementInt` (`self.NumberOfTeamB_Alive`))
        (:`  `
          (if (<= _result_2 0)
            (bind _returnvalue_2 (`|CreateWidget` "/Game/UI/WB_TeamWinner.WB_TeamWinner_C"))
            (`TextBlock.SetText` (`/Game/UI/WB_TeamWinner.WinnerText` _returnvalue_2) "TEAM A WON!")
            (`UserWidget.AddToViewport` _returnvalue_2 0)
            (else
              (goto _label))))))))

(event `UpdateWidget`
  (bind _asbp_third_person_character (cast `/Game/ThirdPerson/Blueprints/BP_ThirdPersonCharacter` (`GameplayStatics.GetPlayerCharacter` 0)))
  (bind _hud (`/Game/ThirdPerson/Blueprints/BP_ThirdPersonCharacter.HUD` _asbp_third_person_character))
  (`TextBlock.SetText` (`/Game/UI/WB_HUD.TeamAText_1` _hud) (`|FormatText` "TEAM A: {VALUE}" (`self.NumberOfTeamA_Alive`)))
  (`TextBlock.SetText` (`/Game/UI/WB_HUD.TeamBText` _hud) (`|FormatText` "TEAM B: {VALUE}" (`self.NumberOfTeamB_Alive`))))

(fn `UserConstructionScript`)