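; Team deathmatch AI soldier that wanders to random reachable points, hunts pawns on the other team and shoots them with a rifle.
; PawnSensing sightings trigger a chase, then a montage notify fires a damaging sphere trace with muzzle and impact effects.
; Damage drains health until the bot ragdolls, hides its widgets and decrements its team count in GS_TeamDeathMatch.
; Tick updates the health bar and turns both widgets toward the camera.
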(event `self.ReceiveBeginPlay`
  (`self.SearchAround`)
  (`|ExecutionSequence`
    (:`then_0`
      (if (== (`self.Team`) 1)
        (bind _aswb_ai_team (cast `/Game/UI/WB_AI_Team` (`WidgetComponent.GetWidget` (`self.TeamWidget`))))
        (bind _teamtext (`/Game/UI/WB_AI_Team.TeamText` _aswb_ai_team))
        (`TextBlock.SetText` _teamtext "TeamB")
        (`TextBlock.SetColorAndOpacity` _teamtext (make `SlateColor` (struct :`R` 1.0 :`B` 0.008304 :`A` 1.0)))))
    (:`then_1`
      (`KismetSystemLibrary.Delay` 0.3 :!label _label)
      (if (`self.bHasSeenTarget?`)
        (`self.SearchAround`)
        (set `self.bHasSeenTarget?` false)
        (goto _label)))))

(event `SearchAround`
  ;[0.05098 0.05098 0.05098] Search Around
  (if (not (`self.bHasSeenTarget?`))
    (`|AIMoveTo` self (`NavigationSystemV1.K2_GetRandomReachablePointInRadius` (`self.K2_GetActorLocation`) 2000.0 null null) null 300.0
      (:`OnSuccess`
        (`KismetSystemLibrary.Delay` 1.0)
        (`self.SearchAround`)))))

(event `self.ReceiveAnyDamage`
  (params (Damage :type "Float (single-precision)") (DamageType :type "DamageType Object Reference") (InstigatedBy :type "Controller Object Reference") (DamageCauser :type "Actor Object Reference"))
  ;[0.05098 0.05098 0.05098] Health
  (set `self.Health` (- (`self.Health`) Damage))
  (if (<= (`self.Health`) 0.0)
    (`/Engine/EditorBlueprintResources/StandardMacros.DoOnce` false
      (:`Completed`
        (`PrimitiveComponent.SetSimulatePhysics` (`self.Mesh`) true)
        (`CharacterMovementComponent.SetMovementMode` (`self.CharacterMovement`) "MOVE_None" 0)
        (set `self.bIsDead?` true)
        (`SceneComponent.SetVisibility` (`self.HealthBarWidget`) false false)
        (`SceneComponent.SetVisibility` (`self.TeamWidget`) false false)
        (bind _asgs_team_death_match (cast `/Game/Blueprints/GS_TeamDeathMatch` (`GameplayStatics.GetGameState`)))
        (`/Game/Blueprints/GS_TeamDeathMatch.DecreaseTeamNumber` _asgs_team_death_match (== (`self.Team`) 0))))))

(event `self.PawnSensing.OnSeePawn`
  (params (Pawn :type "Pawn Object Reference"))
  (if (`KismetSystemLibrary.DoesImplementInterface` Pawn "/Game/Blueprints/BPI_TeamInteraction.BPI_TeamInteraction_C")
    (bind _team (message `/Game/Blueprints/BPI_TeamInteraction.GetTeam` Pawn))
    (if (!= _team (`KismetMathLibrary.Conv_ByteToInt` (`self.Team`)))
      (bind _asbp_ai (cast `/Game/Blueprints/BP_AI` Pawn)
        (:`then`
          (if (`/Game/Blueprints/BP_AI.bIsDead?` _asbp_ai)
            (`self.SearchAround`)
            (else
              (`self.ChaseTarget` Pawn :!label _label_2)
              (set `self.bHasSeenTarget?` true))))
        (:`CastFailed`
          (goto _label_2))))))

(event `ChaseTarget`
  (params (TargetActor :type "Actor Object Reference"))
  (`|AIMoveTo` self (0.0 0.0 0.0) TargetActor 450.0
    (:`OnSuccess`
      (`self.Fire` TargetActor))))

(event `Fire`
  (params (TargetActor :type "Actor Object Reference"))
  (bind _returnvalue_location (`KismetMathLibrary.BreakTransform` (`SceneComponent.GetSocketTransform` (`self.Rifle`) "b_gun_muzzleflash" "RTS_World")))
  (bind _returnvalue (`SceneComponent.K2_GetComponentRotation` (`self.Mesh`)))
  (if (not (`self.bIsDead?`))
    (`Controller.SetControlRotation` (`self.GetController`) (`KismetMathLibrary.FindLookAtRotation` (`self.K2_GetActorLocation`) (`self.K2_GetActorLocation` TargetActor)))
    (`|PlayMontage` (`self.Mesh`) "/Game/ShooterAnimations/Fire_Rifle_Shoot_Montage.Fire_Rifle_Shoot_Montage"
      (:`OnNotifyBegin`
        (`GameplayStatics.SpawnEmitterAttached` "/Game/Realistic_Starter_VFX_Pack_Vol2/Particles/Hit/P_Default.P_Default" (`self.Rifle`) "b_gun_muzzleflash" _returnvalue_location _returnvalue (0.5 0.5 0.5) "KeepWorldPosition")
        (`GameplayStatics.PlaySoundAtLocation` "/Game/Audio/MS_RifleFire.MS_RifleFire" (`self.K2_GetActorLocation`) (struct) 0.65 1.0 0.0 null null null null)
        (bind (_outhit _returnvalue_2) (`KismetSystemLibrary.SphereTraceSingle` _returnvalue_location (+ _returnvalue_location (* (`KismetMathLibrary.GetRightVector` _returnvalue) 3000.0)) 12.0 "TraceTypeQuery1"))
        (if _returnvalue_2
          (bind (_bblockinghit _binitialoverlap _time _distance _location _impactpoint _normal _impactnormal _physmat _hitactor) (`GameplayStatics.BreakHitResult` _outhit))
          (`GameplayStatics.ApplyDamage` _hitactor 5.0)
          (`GameplayStatics.SpawnEmitterAttached` "/Game/Realistic_Starter_VFX_Pack_Vol2/Particles/Hit/P_Default.P_Default" (`self.Rifle`) "b_gun_muzzleflash" _impactpoint (`KismetMathLibrary.MakeRotFromX` _normal) (0.5 0.5 0.5) "KeepWorldPosition")
          (`GameplayStatics.PlaySoundAtLocation` "/Game/Audio/MS_RifleFire.MS_RifleFire" (`self.K2_GetActorLocation`) (struct) 0.65 1.0 0.0 null null null null))))))

(event `self.ReceiveTick`
  (params (DeltaSeconds :type "Float (single-precision)"))
  (bind _aswb_ai_health_bar (cast `/Game/UI/WB_AI_HealthBar` (`WidgetComponent.GetWidget` (`self.HealthBarWidget`))))
  (`ProgressBar.SetPercent` (`/Game/UI/WB_AI_HealthBar.HealthBar` _aswb_ai_health_bar) (/ (`self.Health`) 100.0))
  (`SceneComponent.K2_SetWorldRotation` (`self.HealthBarWidget`) (`KismetMathLibrary.FindLookAtRotation` (`self.K2_GetActorLocation`) (`self.K2_GetActorLocation` (`GameplayStatics.GetPlayerCameraManager` 0))) false false)
  (`SceneComponent.K2_SetWorldRotation` (`self.TeamWidget`) (`KismetMathLibrary.FindLookAtRotation` (`self.K2_GetActorLocation`) (`self.K2_GetActorLocation` (`GameplayStatics.GetPlayerCameraManager` 0))) false false))

(event `/Game/Blueprints/BPI_TeamInteraction.SetTeam`
  (params (Team :type "/Game/Blueprints/E_Teams Enum" :default "NewEnumerator0"))
  (set `self.Team` Team))

(fn `GetTeam`
  (returns (Team :type "/Game/Blueprints/E_Teams Enum"))
  (return (`self.Team`)))

(fn `UserConstructionScript`)